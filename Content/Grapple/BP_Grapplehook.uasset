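; Grapple hook projectile actor that flies in a straight line from its spawn point toward a Target actor.
; On BeginPlay it caches the start and target locations, then sets the ProjectileMovement velocity along the normalized direction at Speed.
; The aim is computed once, so the hook does not track a moving target.
; DistanceToTarget returns the remaining distance to that cached end location.
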(event EventBeginPlay
  (Variables|Private|SetStartingLocation (Transformation|GetActorLocation))
  (Variables|Private|SetEndingLocation (Transformation|GetActorLocation (Variables|Private|GetTarget)))
  (Variables|Private|SetDirection (Math|Vector|Normalize (- (Variables|Private|GetEndingLocation) (Variables|Private|GetStartingLocation))))
  (Variables|/Script/Engine.MovementComponent|SetVelocity (Variables|Default|GetProjectileMovement) (* (Variables|Private|GetDirection) (Variables|Private|GetSpeed))))

(fn ConstructionScript)

(fn DistancetoTarget
  (return (Math|Vector|Distance(Vector) (Variables|Private|GetEndingLocation) (Transformation|GetActorLocation))))