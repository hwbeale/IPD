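; BP_Menu3D is a 3D in-world menu actor that hosts a Menu_Baseclass widget and links to other menus.
; On BeginPlay it binds the widget's transition event and disables its own collision.
; A transition request picks a target from LinkedMenus by index, swaps collision to that menu and blends the player's view to it.
; The blend time and exponent are hardcoded, so TransitionTo's BlendTime input is unused.
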(event Custom|OnTransitionBetweenMenus
  (params (MenuIndex :type Integer))
  (if (Utilities|Array|IsValidIndex (Variables|Default|GetLinkedMenus) MenuIndex)
    (CallFunction|Transitionto (Utilities|Array|Get(acopy) (Variables|Default|GetLinkedMenus) MenuIndex) 0.0)))

(event Custom|TransitionTo
  (params (NewMenu :type BP%20Menu%203D%20Object%20Reference) (BlendTime :type Float%20%28single-precision%29))
  (Collision|SetActorEnableCollision false)
  (Collision|SetActorEnableCollision NewMenu true)
  (Game|Player|SetViewTargetwithBlend (Game|GetPlayerController 0) NewMenu 2.0 "VTBlend_Linear" 5.0 false))

(event EventBeginPlay
  (bind _asmenu_baseclass (Utilities|Casting|CastToMenu_Baseclass (UserInterface|GetUserWidgetObject (Variables|Default|GetWidget))))
  (EventDispatchers|BindEventtoTransitiontoLinkedMenu _asmenu_baseclass (delegate Custom|OnTransitionBetweenMenus))
  (Collision|SetActorEnableCollision false))

(event Collision|EventActorBeginOverlap
  (params (OtherActor :type Actor%20Object%20Reference)))

(event EventTick
  (params (DeltaSeconds :type Float%20%28single-precision%29)))

(fn ConstructionScript)